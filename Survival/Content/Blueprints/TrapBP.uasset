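; Trap actor that snares an overlapping SThirdPersonChar while IsActive is set.
; The construction script creates a dynamic material instance from TrapInst.
; Every tick, the floored TrapState picks green, orange or a default red for its InputColour parameter and reapplies the material to the Sphere.
; Nothing in these graphs changes IsActive or TrapState.
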(event EventBeginPlay)

(event EventActorBeginOverlap
  (params (OtherActor :type Actor%20Object%20Reference))
  (if (Variables|Default|GetisActive)
    (bind _assthird_person_char (Utilities|Casting|CastToSThirdPersonChar OtherActor))
    (Default|Snare _assthird_person_char)))

(event EventTick
  (params (DeltaSeconds :type Float%20%28single-precision%29))
  (switch int (Math|Float|Floor (Variables|Default|GettrapState))
    (:Default
      (Rendering|Material|SetVectorParameterValue (Variables|Default|GetThisTrap) "InputColour" "(R=1.000000,G=0.000000,B=0.000000,A=1.000000)" :!class /Script/Engine.MaterialInstanceDynamic :!label _label)
      (Rendering|Material|SetMaterial (Variables|Default|GetSphere) 0 (Variables|Default|GetThisTrap)))
    (:0
      (Rendering|Material|SetVectorParameterValue (Variables|Default|GetThisTrap) "InputColour" "(R=0.000000,G=1.000000,B=0.056943,A=1.000000)" :!class /Script/Engine.MaterialInstanceDynamic)
      (Rendering|Material|SetMaterial (Variables|Default|GetSphere) 0 (Variables|Default|GetThisTrap)))
    (:1
      (goto _label))
    (:2
      (Rendering|Material|SetVectorParameterValue (Variables|Default|GetThisTrap) "InputColour" "(R=1.000000,G=0.562032,B=0.037451,A=1.000000)" :!class /Script/Engine.MaterialInstanceDynamic)
      (Rendering|Material|SetMaterial (Variables|Default|GetSphere) 0 (Variables|Default|GetThisTrap)))))

(fn ConstructionScript
  (bind _returnvalue (Rendering|Material|CreateDynamicMaterialInstance 0 "/Game/Materials/TrapInst.TrapInst" :!class /Script/Engine.KismetMaterialLibrary))
  (Variables|Default|SetThisTrap _returnvalue))